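; Game board actor for a Scrabble-style word game that spawns a square grid of BP_GridSpace tiles on BeginPlay.
; Each tile receives its index, and a branch chain on its row and column picks a bonus material for star, word-score or letter-score squares.
; The pattern is mostly derived from BoardSize, with some hard-coded coordinates.
; Only materials mark the bonuses; no point multipliers are set.
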(event `self.ReceiveBeginPlay`
  (bind _board_size (`self.Board_Size`))
  (bind _board_size_2 (`self.Board_Size`))
  (bind _y_coord (`self.Y_Coord`))
  (bind _y_coord_2 (`self.Y_Coord`))
  (bind _x_coord (`self.X_Coord`))
  (bind _y_coord_3 (`self.Y_Coord`))
  (bind _board_size_3 (`self.Board_Size`))
  (bind _x_coord_2 (`self.X_Coord`))
  (bind _x_coord_3 (`self.X_Coord`))
  (bind _x_coord_4 (`self.X_Coord`))
  (bind _y_coord_4 (`self.Y_Coord`))
  (bind _y_coord_5 (`self.Y_Coord`))
  (bind _y_coord_6 (`self.Y_Coord`))
  (bind _board_size_4 (`self.Board_Size`))
  (bind _y_coord_7 (`self.Y_Coord`))
  (bind _x_coord_5 (`self.X_Coord`))
  (bind _returnvalue (/ (`self.Board_Size`) 2))
  (bind _returnvalue_2 (/ (`self.Board_Size`) 2))
  (bind _returnvalue_3 (/ (`self.Board_Size`) 2))
  (bind _returnvalue_4 (/ (`self.Board_Size`) 2))
  (bind _returnvalue_5 (/ _board_size_4 2))
  (bind _returnvalue_6 (- _board_size_4 1))
  (bind _returnvalue_7 (not (and (== _returnvalue_5 _y_coord_6) (== _returnvalue_5 _x_coord_5))))
  (bind _returnvalue_8 (and (or (== _y_coord_6 0) (== _y_coord_6 _returnvalue_5) (== _y_coord_6 _returnvalue_6)) (or (== _x_coord_5 0) (== _x_coord_5 _returnvalue_5) (== _x_coord_5 _returnvalue_6))))
  (for _index (range (* _board_size _board_size))
    (bind _returnvalue_9 (/ _index _board_size_2))
    (set `self.X_Coord` _returnvalue_9)
    (bind _returnvalue_10 (mod _index _board_size_2))
    (set `self.Y_Coord` _returnvalue_10)
    (bind _returnvalue_11 (`|SpawnActorFromClass` "/Game/Upwards-Actors/BP_GridSpace.BP_GridSpace_C" (`KismetMathLibrary.MakeTransform` (`KismetMathLibrary.MakeVector` (* _returnvalue_10 400.0) (* _returnvalue_9 400.0))) "Undefined" "OverrideRootScale" null 0 null))
    (set `/Game/Upwards-Actors/BP_GridSpace.Index` _index _returnvalue_11)
    (if (and _returnvalue_8 _returnvalue_7)
      (bind _gridspacemesh (`/Game/Upwards-Actors/BP_GridSpace.GridSpaceMesh` _returnvalue_11))
      (`PrimitiveComponent.SetMaterial` _gridspacemesh 0 "/Game/tiles/Triple__Word_Score_Mat.Triple__Word_Score_Mat")
      (elif (`KismetMathLibrary.BooleanNAND` (not _returnvalue_8) _returnvalue_7)
        (`PrimitiveComponent.SetMaterial` _gridspacemesh 0 "/Game/tiles/star_Mat.star_Mat")
        (elif (or (== (`self.Y_Coord`) (`self.X_Coord`)) (== (`self.Y_Coord`) (- (- (`self.Board_Size`) 1) (`self.X_Coord`))))
          (if (or (== _returnvalue_2 (+ _y_coord_2 1)) (== (- _y_coord_2 1) _returnvalue_2))
            (`PrimitiveComponent.SetMaterial` _gridspacemesh 0 "/Game/tiles/double_letter_score_Mat.double_letter_score_Mat")
            (elif (or (== _returnvalue (+ _y_coord 2)) (== (- _y_coord 2) _returnvalue))
              (`PrimitiveComponent.SetMaterial` _gridspacemesh 0 "/Game/tiles/triple_letter_score_mat.triple_letter_score_Mat")
              (else
                (`PrimitiveComponent.SetMaterial` _gridspacemesh 0 "/Game/tiles/Double_word_score_Mat.Double_word_score_Mat"))))
          (elif (and (or (== _y_coord_3 5) (== _y_coord_3 9)) (or (== _x_coord 1) (== _x_coord 5) (== _x_coord 9) (== _x_coord 13)))
            (`PrimitiveComponent.SetMaterial` _gridspacemesh 0 "/Game/tiles/triple_letter_score_mat.triple_letter_score_Mat")
            (elif (and (or (== _x_coord_3 0) (== _x_coord_3 (- (`self.Board_Size`) 1))) (or (== _y_coord_5 (+ _returnvalue_4 4)) (== _y_coord_5 (- _returnvalue_4 4))))
              (`PrimitiveComponent.SetMaterial` _gridspacemesh 0 "/Game/tiles/double_letter_score_Mat.double_letter_score_Mat" :!label _label)
              (elif (and (or (== _x_coord_4 2) (== _x_coord_4 (- (`self.Board_Size`) 3))) (or (== _y_coord_4 (+ _returnvalue_3 1)) (== _y_coord_4 (- _returnvalue_3 1))))
                (goto _label)
                (elif (and (or (== _x_coord_2 3) (== _x_coord_2 (- (`self.Board_Size`) 4))) (or (== _y_coord_7 0) (== _y_coord_7 (/ _board_size_3 2)) (== _y_coord_7 (- _board_size_3 1))))
                  (goto _label))))))))))

(event `self.ReceiveActorOnClicked`
  (params (ButtonPressed :type "Key Structure")))

(fn `UserConstructionScript`)