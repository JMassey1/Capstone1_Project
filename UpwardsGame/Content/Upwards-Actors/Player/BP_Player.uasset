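; BP_Player holds the player's tile hand and score for a letter-tile word game.
; On BeginPlay it draws seven tiles from Mouse_GameMode into the TileHand map, triggers the hand UI and prints debug counts.
; DrawATile only caches the game mode; its logic for adding a drawn tile is disconnected.
; UpdateScore adds the Points of whichever BP_GridSpace GetActorOfClass returns to Score.
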(event `self.ReceiveBeginPlay`
  (bind _tilehand (`self.TileHand`))
  (bind _asmouse_game_mode (cast `/Game/Mouse_GameMode` (`GameplayStatics.GetGameMode`)))
  (set `self.GameMode` _asmouse_game_mode)
  (bind _returnedhand (`/Game/Mouse_GameMode.DrawHand` _asmouse_game_mode 7))
  (bind _output_get (set `self.TileHand` _returnedhand))
  (`self.TriggerDrawUI` _output_get)
  (`KismetSystemLibrary.PrintString` "called trigger")
  (for _index (range (`BlueprintMapLibrary.Map_Length` _tilehand))
    (bind _keys (`BlueprintMapLibrary.Map_Keys` _tilehand))
    (bind _values (`BlueprintMapLibrary.Map_Values` _tilehand))
    (`KismetSystemLibrary.PrintString` (`KismetStringLibrary.Concat_StrStr` "Given: " (`KismetStringLibrary.Conv_IntToString` (`|GetArrayItem` _values _index)) " " (`KismetStringLibrary.Conv_ObjectToString` (`|GetArrayItem` _keys _index)) " tile(s)") true true (struct :`R` 0.1388 :`G` 1.0 :`B` 0.105379 :`A` 1.0) 3.0)))

(event `DrawATile`
  (bind _asmouse_game_mode (cast `/Game/Mouse_GameMode` (`GameplayStatics.GetGameMode`)))
  (set `self.GameMode` _asmouse_game_mode))

(fn `update_score`
  (bind _returnvalue (`GameplayStatics.GetActorOfClass` "/Game/Upwards-Actors/BP_GridSpace.BP_GridSpace_C"))
  (set `self.score` (+ (`self.score`) (`/Game/Upwards-Actors/BP_GridSpace.points` _returnvalue))))

(fn `UserConstructionScript`)