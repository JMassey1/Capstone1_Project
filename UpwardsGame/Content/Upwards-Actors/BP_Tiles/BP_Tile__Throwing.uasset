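; Lettered tile actor that the player aims and throws from a fixed launch point.
; Holding right mouse with the turn axes rotates the box; left click launches it with physics at a set velocity.
; A throw disables input and switches from the follow camera to a stationary one, then resets everything after five seconds.
; BeginPlay sets the letter and performs a brief throw-and-reset to work around uncontrolled spinning.
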(event `self.ReceiveBeginPlay`
  (bind _stay_camera (`self.stay_camera`))
  (bind _box (`self.Box`))
  (bind _box_2 (`self.Box`))
  ;[1 1 1] sets the text on the tile
  (`TextRenderComponent.K2_SetText` (`self.LetterRender`) (`KismetTextLibrary.Conv_StringToText` (`self.Letter`)))
  ;[1 1 1] does a throw event because for some reason if there is not one the tile sits there and spins like crazy
  (`self.theThrowEvent`)
  (`KismetSystemLibrary.Delay` 0.1)
  (`PrimitiveComponent.SetPhysicsLinearVelocity` _box_2 (0.0 0.0 0.0) false "None")
  (`PrimitiveComponent.SetSimulatePhysics` _box_2 false)
  (`SceneComponent.K2_SetWorldLocationAndRotation` _box_2 (2820.0 -2410.0 2040.0) (struct :`Pitch` 90.0 :`Yaw` 180.0 :`Roll` 90.0) false false)
  ;[1 1 1] sets the camera that watches the tile fly in a specific location
  (`SceneComponent.K2_SetWorldLocation` _stay_camera (-2200.0 2770.0 2600.0) false false)
  (`SceneComponent.K2_SetWorldRotation` _stay_camera (struct :`Pitch` -23.0) false false)
  ;[1 1 1] this should be what causes the tile to rotate. Rotates very wonky though and not sure why
  (if (`PlayerController.IsInputKeyDown` (`GameplayStatics.GetPlayerController` 0) "RightMouseButton")
    (`SceneComponent.K2_SetWorldRotation` _box (`KismetMathLibrary.ComposeRotators` (`SceneComponent.RelativeRotation` _box) (`KismetMathLibrary.MakeRotator` (* (stale `InputAxis|turn_ver` AxisValue) -1.0) 0.0 (* (stale `InputAxis|turn_hor` AxisValue) 1.0))) false false :!label _label)))

(event `InputAxis|turn_ver`
  (params (AxisValue :type "Float (single-precision)"))
  ;[1 1 1] this should be what causes the tile to rotate. Rotates very wonky though and not sure why
  (goto _label))

(event `InputAxis|turn_hor`
  (params (AxisValue :type "Float (single-precision)"))
  ;[1 1 1] this should be what causes the tile to rotate. Rotates very wonky though and not sure why
  (goto _label))

(event `Key|LeftMouseButton`
  (params (Key :type "Key Structure"))
  (bind _box (`self.Box`))
  ;[1 1 1] when left mouse button is clicked the tile is thrown and control is taken away from the user. The camera that watches the tile fly is then active and the carema that follows the tile is not active
  (:`Pressed`
    (`self.theThrowEvent`)
    (`self.DisableInput` (`ActorComponent.GetOwner` (`self.Box`)) (`GameplayStatics.GetPlayerController` 0))
    (`ActorComponent.SetActive` (`self.stay_camera`) true false)
    (`ActorComponent.SetActive` (`self.follow_Camera`) false false)
    ;[1 1 1] after a 5 second delay the tile is then reset to its launching position, the tile camera is active and the camera that watches the tile fly is not active, and control is given back to the player
    (`KismetSystemLibrary.Delay` 5.0)
    (`PrimitiveComponent.SetPhysicsLinearVelocity` _box (0.0 0.0 0.0) false "None")
    (`PrimitiveComponent.SetSimulatePhysics` _box false)
    (`SceneComponent.K2_SetWorldLocationAndRotation` _box (2820.0 -2410.0 2040.0) (struct :`Pitch` 90.0 :`Yaw` 180.0 :`Roll` 90.0) false false)
    (`ActorComponent.SetActive` (`self.follow_Camera`) true false)
    (`ActorComponent.SetActive` (`self.stay_camera`) false false)
    (`self.EnableInput` (`ActorComponent.GetOwner` (`self.Box`)) (`GameplayStatics.GetPlayerController` 0))))

(event `theThrowEvent`
  (bind _box (`self.Box`))
  ;[1 1 1] Should be the function to click the tile to throw it, has a set velocity because for some reason it would not let me let the user hold space bar to tell it how far to fly
  (`PrimitiveComponent.SetSimulatePhysics` _box true)
  (`PrimitiveComponent.SetPhysicsLinearVelocity` _box (+ (* (`SceneComponent.GetUpVector` _box) -4000.0) (* (`SceneComponent.GetForwardVector` _box) 500.0)) false "None"))

(fn `DestroyTile`
  (`self.K2_DestroyActor` self))

(fn `Right Click Launch1`)

(fn `SetLetter`
  (params (NewLetter :type String))
  (`TextRenderComponent.K2_SetText` (`self.LetterRender`) (`KismetTextLibrary.Conv_StringToText` NewLetter)))

(fn `UserConstructionScript`)