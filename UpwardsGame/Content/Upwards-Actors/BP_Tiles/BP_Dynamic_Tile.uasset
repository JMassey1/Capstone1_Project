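; BP_Dynamic_Tile is a clickable letter tile that shows a letter and its point value.
; BeginPlay writes the Letter and Points variables to two text renders, and SetLetter later changes only the displayed letter.
; Clicking the cube prints a debug message and asks the parent grid space to remove the tile.
; DestroyTile destroys the actor.
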(event `self.ReceiveBeginPlay`
  (`TextRenderComponent.K2_SetText` (`self.LetterRender`) (`KismetTextLibrary.Conv_StringToText` (`self.Letter`)))
  (`TextRenderComponent.K2_SetText` (`self.ScoreRender`) (`KismetTextLibrary.Conv_IntToText` (`self.Points`))))

(event `self.Cube.OnClicked`
  (params (TouchedComponent :type "PrimitiveComponent Object Reference") (ButtonPressed :type "Key Structure"))
  (`KismetSystemLibrary.PrintString` "Deleting Tile")
  (`/Game/Upwards-Actors/BP_GridSpace.RemoveTile` (`self.ParentGridSpace`)))

(fn `DestroyTile`
  (`self.K2_DestroyActor` self))

(fn `SetLetter`
  (params (NewLetter :type String))
  (`TextRenderComponent.K2_SetText` (`self.LetterRender`) (`KismetTextLibrary.Conv_StringToText` NewLetter)))

(fn `UserConstructionScript`)