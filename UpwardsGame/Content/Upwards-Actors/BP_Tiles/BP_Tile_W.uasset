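; BP_Tile_W is a letter tile actor, by its name the W tile, that displays a letter and its point score.
; On BeginPlay it writes its Letter and Points variables to two text render components.
; Clicking the Cube component destroys the tile and prints a debug message.
; SetLetter changes only the displayed text, and DestroyTile also removes the actor.
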(event `self.ReceiveBeginPlay`
  (`TextRenderComponent.K2_SetText` (`self.LetterRender`) (`KismetTextLibrary.Conv_StringToText` (`self.Letter`)))
  (`TextRenderComponent.K2_SetText` (`self.ScoreRender`) (`KismetTextLibrary.Conv_IntToText` (`self.Points`))))

(event `self.Cube.OnClicked`
  (params (TouchedComponent :type "PrimitiveComponent Object Reference") (ButtonPressed :type "Key Structure"))
  (`self.K2_DestroyActor`)
  (`KismetSystemLibrary.PrintString` "Deleting Tile"))

(fn `DestroyTile`
  (`self.K2_DestroyActor` self))

(fn `SetLetter`
  (params (NewLetter :type String))
  (`TextRenderComponent.K2_SetText` (`self.LetterRender`) (`KismetTextLibrary.Conv_StringToText` NewLetter)))

(fn `UserConstructionScript`)