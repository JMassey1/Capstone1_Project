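; BP_DoubleWordPower is a powerup actor, named for a double-word bonus, that is triggered when a thrown tile hits its cube.
; On a hit from BP_Tile__Throwing it destroys the cube, enables input and shows a PowerupTextDisplay widget with its PowerupText.
; After a short delay it removes the widget and destroys itself; the graph applies no scoring effect.
; The construction script resets the cube's relative location to the origin.
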(event `self.Cube.OnComponentHit`
  (params (HitComponent :type "PrimitiveComponent Object Reference") (OtherActor :type "Actor Object Reference") (OtherComp :type "PrimitiveComponent Object Reference") (NormalImpulse :type "Vector Structure") (Hit :type "HitResult Structure (by ref)"))
  (cast `/Game/Upwards-Actors/BP_Tiles/BP_Tile__Throwing` OtherActor)
  (`ActorComponent.K2_DestroyComponent` (`self.Cube`))
  (`self.EnableInput` null)
  (bind _returnvalue (`|CreateWidget` "/Game/PowerupTextDisplay.PowerupTextDisplay_C"))
  (set `/Game/PowerupTextDisplay.PowerupText` (`self.Powerup Text`) _returnvalue)
  (`UserWidget.AddToViewport` _returnvalue 0)
  (`KismetSystemLibrary.Delay` 2.0)
  (`Widget.RemoveFromParent` _returnvalue)
  (`self.K2_DestroyActor`))

(fn `UserConstructionScript`
  (`SceneComponent.K2_SetRelativeLocation` (`self.Cube`) (0.0 0.0 0.0) false false))