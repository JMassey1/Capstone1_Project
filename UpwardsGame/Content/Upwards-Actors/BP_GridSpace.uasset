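; One clickable cell on the Upwards word-game board that places and removes letter tiles.
; Clicking an empty cell has the GameMode spawn a tile and registers the cell in BP_UpwardsBoard's overall and per-turn lists.
; The first tile requires the center cell (Index 112); later ones need an orthogonal neighbor and the row or column set by the turn's second tile.
; RemoveTile unregisters the cell and returns its letter or wildcard to the current player.
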(event `self.ReceiveBeginPlay`
  (bind _asmouse_game_mode (cast `/Game/Mouse_GameMode` (`GameplayStatics.GetGameMode`)))
  (set `self.GameMode` _asmouse_game_mode))

(event `self.GridSpaceMesh.OnClicked`
  (params (TouchedComponent :type "PrimitiveComponent Object Reference") (ButtonPressed :type "Key Structure"))
  (if (`self.hasTile`)
    _
    (elif (`/Game/Mouse_GameMode.IsFirstTilePlaced` (stale `self.ReceiveBeginPlay` _asmouse_game_mode))
      (bind _is_valid (`self.isValidOnBoard`))
      (bind _isvalid (`self.Is Valid on Turn`))
      (`KismetSystemLibrary.PrintString` (`KismetStringLibrary.Conv_BoolToString` _isvalid) true true (struct :`G` 0.66 :`B` 1.0 :`A` 1.0) 5.0)
      (if (and _isvalid _is_valid)
        (bind _newparam (`/Game/Mouse_GameMode.CreateTile` (`self.GameMode`) (`KismetMathLibrary.MakeTransform` (+ (`self.K2_GetActorLocation`) (0.0 0.0 20.0)) (struct) (3.0 3.0 3.0)) self :!label _label))
        (set `self.currTile` _newparam)
        (set `self.hasTile` true)
        (`KismetSystemLibrary.PrintText` "Placing Tile")
        (bind _returnvalue (`GameplayStatics.GetActorOfClass` "/Game/Upwards-Actors/BP_UpwardsBoard.BP_UpwardsBoard_C"))
        (`KismetArrayLibrary.Array_Add` (`/Game/Upwards-Actors/BP_UpwardsBoard.placed_tiles` _returnvalue) self)
        (`KismetArrayLibrary.Array_Add` (`/Game/Upwards-Actors/BP_UpwardsBoard.placed_tiles_turn` _returnvalue) self)
        (`KismetSystemLibrary.PrintString` "ADDED SHIT"))
      (elif (== (`self.Index`) 112)
        (set `/Game/Mouse_GameMode.IsFirstTilePlaced` true (stale `self.ReceiveBeginPlay` _asmouse_game_mode))
        (goto _label)
        (else
          (`KismetSystemLibrary.PrintString` "MUST PLACE TILE ON CENTER FIRST"))))))

(event `RemoveTile`
  (bind _currtile (`self.currTile`))
  (bind _player (`/Game/Mouse_GameMode.GetCurrentPlayer` (`self.GameMode`)))
  (bind _returnvalue (`GameplayStatics.GetActorOfClass` "/Game/Upwards-Actors/BP_UpwardsBoard.BP_UpwardsBoard_C"))
  (bind _placed_tiles_turn (`/Game/Upwards-Actors/BP_UpwardsBoard.placed_tiles_turn` _returnvalue))
  (`KismetArrayLibrary.Array_Remove` _placed_tiles_turn (`KismetArrayLibrary.Array_Find` _placed_tiles_turn self))
  (bind _placed_tiles (`/Game/Upwards-Actors/BP_UpwardsBoard.placed_tiles` _returnvalue))
  (`KismetArrayLibrary.Array_Remove` _placed_tiles (`KismetArrayLibrary.Array_Find` _placed_tiles self))
  (if (`/Game/Upwards-Actors/BP_Tiles/BP_Dynamic_Tile.wasWild` (`self.currTile`))
    (`/Game/Upwards-Actors/Player/BP_Player.ReturnTile` _player "_")
    (else
      (`/Game/Upwards-Actors/Player/BP_Player.ReturnTile` _player (`/Game/Upwards-Actors/BP_Tiles/BP_Dynamic_Tile.Letter` _currtile))))
  (`self.K2_DestroyActor` _currtile)
  (set `self.hasTile` false)
  (if (== (`KismetArrayLibrary.Array_Length` _placed_tiles) 0)
    (set `/Game/Mouse_GameMode.IsFirstTilePlaced` false (`self.GameMode`))))

(event `PlaceTile`
  (params (TileActor :type "Object Object Reference")))

(event `RightClickTEST`
  (`KismetSystemLibrary.PrintText` "RIGHT MOUSE BUTTON"))

(fn `CanPlaceTile`
  (returns (CanPlace :type Boolean))
  (bind _return (`self.IsFirstTilePlaced`))
  (return _return))

(fn `Is Valid on Turn`
  (returns (isValid :type Boolean))
  (locals (CurrX :type Integer) (CurrY :type Integer))
  (bind _parentboard (`self.ParentBoard`))
  (bind _initialdisplacementdirection (`/Game/Upwards-Actors/BP_UpwardsBoard.initialDisplacementDirection` _parentboard))
  (bind _returnvalue (`KismetArrayLibrary.Array_Length` (`/Game/Upwards-Actors/BP_UpwardsBoard.placed_tiles_turn` (`self.ParentBoard`))))
  (bind _output (`|GetArrayItem` (`/Game/Upwards-Actors/BP_UpwardsBoard.placed_tiles_turn` (`self.ParentBoard`))))
  (bind _output_2 (`|GetArrayItem` (`/Game/Upwards-Actors/BP_UpwardsBoard.placed_tiles_turn` (`self.ParentBoard`))))
  (bind _returnvalue_2 (== (`/Game/Upwards-Actors/BP_GridSpace.X_Coord` _output_2) (`self.X_Coord`)))
  (bind _returnvalue_3 (== (`/Game/Upwards-Actors/BP_GridSpace.Y_Coord` _output_2) (`self.Y_Coord`)))
  (`KismetSystemLibrary.PrintString` (`KismetStringLibrary.Concat_StrStr` "Validating Length: " (`KismetStringLibrary.Conv_IntToString` _returnvalue)) true false (struct :`G` 0.66 :`B` 1.0 :`A` 1.0) 5.0)
  (if (== _returnvalue 1)
    (if (== (`/Game/Upwards-Actors/BP_GridSpace.X_Coord` _output) (`self.X_Coord`))
      (if (== (`/Game/Upwards-Actors/BP_GridSpace.Y_Coord` _output) (`self.Y_Coord`))
        (`KismetSystemLibrary.PrintString` "ERROR IN VALID TURN" false false)
        (else
          (set `/Game/Upwards-Actors/BP_UpwardsBoard.initialDisplacementDirection` "Y" _parentboard)
          (return true)))
      (else
        (set `/Game/Upwards-Actors/BP_UpwardsBoard.initialDisplacementDirection` "X" _parentboard)
        (return true)))
    (elif (> _returnvalue 1)
      (`KismetSystemLibrary.PrintString` (`KismetStringLibrary.Concat_StrStr` "Displacement: " _initialdisplacementdirection) false false (struct :`G` 0.66 :`B` 1.0 :`A` 1.0) 5.0)
      (switch `string` _initialdisplacementdirection
        (:`X`
          (return (and (not _returnvalue_2) _returnvalue_3)))
        (:`Y`
          (return (and _returnvalue_2 (not _returnvalue_3)))))
      (else
        (`KismetSystemLibrary.PrintString` "FOUND THE PROBLEM" false false)
        (return true)))))

(fn `IsFirstTilePlaced`
  (returns (Return :type Boolean))
  (return (`/Game/Mouse_GameMode.IsFirstTilePlaced` (`self.GameMode`))))

(fn `isValidOnBoard`
  (returns (is_valid :type Boolean))
  (bind _x_coord (`self.X_Coord`))
  (bind _y_coord (`self.Y_Coord`))
  (set `self.Cur X` _x_coord)
  (set `self.Cur Y` _y_coord)
  (bind _returnvalue (`GameplayStatics.GetActorOfClass` "/Game/Upwards-Actors/BP_UpwardsBoard.BP_UpwardsBoard_C"))
  (for _array_element (`/Game/Upwards-Actors/BP_UpwardsBoard.placed_tiles` _returnvalue)
    (bind _x_coord_2 (`/Game/Upwards-Actors/BP_GridSpace.X_Coord` _array_element))
    (bind _y_coord_2 (`/Game/Upwards-Actors/BP_GridSpace.Y_Coord` _array_element))
    (`KismetSystemLibrary.PrintString` (`KismetStringLibrary.Concat_StrStr` "Testing if tile (x:" (`KismetStringLibrary.Conv_IntToString` _x_coord) ", y:" (`KismetStringLibrary.Conv_IntToString` _y_coord) ") is near tile (x: " (`KismetStringLibrary.Conv_IntToString` _x_coord_2) ",y: " (`KismetStringLibrary.Conv_IntToString` _y_coord_2) ")") false false)
    (if (and (== _y_coord_2 (`self.Cur Y`)) (== (`self.Cur X`) (+ _x_coord_2 1)))
      (while false
        _)
      (return true)
      (elif (and (== _y_coord_2 (`self.Cur Y`)) (== (`self.Cur X`) (+ -1 _x_coord_2)))
        (while false
          _)
        (return true)
        (elif (and (== (+ (`self.Cur Y`) 1) _y_coord_2) (== (`self.Cur X`) _x_coord_2))
          (while false
            _)
          (return true)
          (elif (and (== (+ (`self.Cur Y`) -1) _y_coord_2) (== (`self.Cur X`) _x_coord_2))
            (while false
              _)
            (return true))))))
  (return false) ; Return False if the loop completes without a match
)

(fn `UserConstructionScript`)